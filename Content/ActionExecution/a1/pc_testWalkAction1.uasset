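; Prototype player-character actor that walks toward a travel destination in simulation time rather than frame time.
; A declared-travel event stores a path, and each sim tick accumulates tracked time, runs walking, then reports completion to the sim manager.
; Walking steps by walk speed times tick seconds toward only the first path point, teleporting each step, then snaps there and signals ReachedDestination.
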(event `self.ExecuteSimTick`
  (params (simStep :type "Timespan Structure"))
  (`self.handleSimTick` simStep) ; inside a function so it's trivial to ensure callback runs in blueprint def. Handling a sim tick SHOULDNT be asyncronous. (currently)
  (`SimManaged.SimTickCompleted` (`self.SimManaged`)))

(event `Player declared 'Travel down  the road`
  (params (path :type "Array of Vector Structure"))
  ; Hacky implementation for handling an action
  (set `self.path` path)
  (set `self.havePathToTravel` true))

(fn `handleSimTick`
  (params (simStep :type "Timespan Structure"))
  (locals (NewLocalVar :type "Timespan Structure"))
  (bind _output_get (set `self.trackedSimTime` (+ (`self.trackedSimTime`) (`KismetMathLibrary.FromMilliseconds` (`KismetMathLibrary.GetTotalMilliseconds` simStep)))))
  (`KismetSystemLibrary.PrintText` (`|FormatText` "simtime passed in seconds {1}" (`KismetMathLibrary.GetTotalSeconds` _output_get)))
  ; again, bad way to define. but passable for prototype
  (if (`self.havePathToTravel`)
    (`self.handlingWalking` simStep)))

(fn `handlingWalking`
  (params (NewParam :type "Timespan Structure"))
  (locals (NewLocalVar_0 :type "Vector Structure") (NewLocalVar_1 :type "Vector Structure") (NewLocalVar_2 :type "Vector Structure"))
  (bind _location (.location (`self.GetTransform`)))
  (bind _output (`|GetArrayItem` (`self.path`)))
  (bind _returnvalue (* (`self.WalkSpeed`) (`KismetMathLibrary.GetTotalSeconds` NewParam)))
  (bind _output_get (set `local.NewLocalVar_0` (`KismetMathLibrary.GetDirectionUnitVector` _location _output)))
  (bind _output_get_2 (set `local.NewLocalVar_1` (* _output_get _returnvalue)))
  (bind _output_get_3 (set `local.NewLocalVar_2` (+ _location _output_get_2)))
  (if (>= (`KismetMathLibrary.Vector_Distance` _output _location) _returnvalue)
    (`self.K2_SetActorLocation` _output_get_3 false true) ; this impl will overshoot abit. We need to detect if within threshold
    (else
      (`KismetSystemLibrary.PrintText` (`|FormatText` "pc reached destination at sim time {1}" (`KismetMathLibrary.GetTotalSeconds` (`self.trackedSimTime`))))
      (`self.K2_SetActorLocation` _output false true)
      ; this ends up being a bit inaccurate. we really need to call an interrupt on sim manager at this point because of thread execution
      (set `self.havePathToTravel` false)
      (`self.reachedDestination`))))

(fn `NewFunction`)

(fn `UserConstructionScript`)