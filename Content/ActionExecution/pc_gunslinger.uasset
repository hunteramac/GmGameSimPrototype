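; Player-character (PC) gunslinger Blueprint that simulates declared walk actions the way a game master would, as straight moves across unblocked floor without physics.
; SetAction passes the action's vector to WalkAcrossUnblockedFloor, which derives travel time from distance and speed in meters per second.
; Tick lerps position with teleporting moves and prints progress until arrival.
; An unconfigured AIMoveTo event and disconnected navmesh pathfinding nodes remain as alternative movement experiments.
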(event `self.ReceiveBeginPlay`)

(event `SetAction`
  (params (newAction :type "/Game/ActionExecution/S_DeclaredActionInfo Structure"))
  (bind _output_get (set `self.NewVar` newAction))
  (`self.WalkAcrossUnblockedFloor` (`.vector_9_1F2F39224FEA6891A2DA49AA292CA469` (break `/Game/ActionExecution/S_DeclaredActionInfo` _output_get))))

(event `WalkAcrossUnblockedFloor`
  (params (MoveInput :type "Vector Structure (by ref)"))
  (bind _location (.location (`self.GetTransform`)))
  (set `self.endPos` MoveInput)
  (set `self.startPos` _location)
  (set `self.timeToGettoEndPos` (/ (`KismetMathLibrary.Vector_Distance` _location MoveInput) (* (`self.speed_MetersPerSecond`) 100.0)))
  (set `self.curTime` 0.0)
  (set `self.walkingToPos` true))

(event `self.ReceiveTick`
  (params (DeltaSeconds :type "Float (single-precision)"))
  (bind _endpos (`self.endPos`))
  (bind _curtime (`self.curTime`))
  (bind _timetogettoendpos (`self.timeToGettoEndPos`))
  (bind _returnvalue (/ _curtime _timetogettoendpos))
  (if (`self.walkingToPos`)
    (set `self.curTime` (+ DeltaSeconds (`self.curTime`)))
    (if (>= _returnvalue 1.0)
      (set `self.walkingToPos` false)
      (`self.K2_SetActorLocationAndRotation` _endpos (struct) false true)
      (else
        (`self.K2_SetActorLocationAndRotation` (`KismetMathLibrary.VLerp` (`self.startPos`) _endpos _returnvalue) (struct) false true) ; We should trigger any events, before moving again.
        (`KismetSystemLibrary.PrintText` (`|FormatText` "{1} {2}" _curtime _timetogettoendpos) true true (struct :`G` 0.66 :`B` 1.0 :`A` 1.0) _returnvalue)))))

(event `PhysiscsMove`
  (`|AIMoveTo` null (0.0 0.0 0.0) null))

(fn `UserConstructionScript`)