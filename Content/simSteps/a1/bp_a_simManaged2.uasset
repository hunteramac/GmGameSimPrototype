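; Actor that takes part in a stepped simulation managed by a controller, running its work whenever a sim step starts.
; On BeginPlay it loops until the player controller is valid, casts it and binds a custom event to the controller's sim-step start.
; That event calls HandleSimStep, and a step-completed event reports back to the controller, passing itself as the responder.
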(event `self.ReceiveBeginPlay`
  (bind _returnvalue (`GameplayStatics.GetPlayerController` 0))
  (while (not (`KismetSystemLibrary.IsValid` _returnvalue))
    _)
  (bind _ascontroller (cast `/Game/Controller` _returnvalue))
  (set `self.As Controller` _ascontroller)
  (add `/Game/Controller.simStepStart` _ascontroller (delegate `CustomEvent`)))

(event `CustomEvent`
  (`self.HandleSimStep`))

(event `SimStep completed`
  (`/Game/Controller.ResponseFromSimMananged` (`self.As Controller`) self))