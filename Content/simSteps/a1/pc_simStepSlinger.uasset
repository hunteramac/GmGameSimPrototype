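; Player-character simulation-step handler that walks its actor to a requested point on simulation time.
; BeginPlay caches the Controller and binds SimTick to the SimManaged2 step event; DoWalkToPoint only stores the target and flags a start.
; The next tick records start position and time, then later ticks lerp at constant speed by elapsed CurSimTime, ignoring collisions.
; Every tick prints sim time and reports SimStepCompleted back to SimManaged2.
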(event `self.ReceiveBeginPlay`
  (bind _returnvalue (`GameplayStatics.GetPlayerController` 0))
  (while (not (`KismetSystemLibrary.IsValid` _returnvalue))
    _)
  (bind _ascontroller (cast `/Game/Controller` _returnvalue))
  (set `self.As Controller` _ascontroller)
  (add `/Game/simSteps/a1/simManaged2.HandleSimStep` (`self.simManaged2`) (delegate `Sim Tick`)))

(event `Sim Tick`
  (bind _as_controller (`self.As Controller`))
  (bind _go_to (`self.Go To`))
  (bind _cursimtime (`/Game/Controller.curSimTime` _as_controller))
  (`KismetSystemLibrary.PrintText` (`|FormatText` "simTime in seconds: {1}" (`KismetMathLibrary.FTrunc` (`KismetMathLibrary.GetTotalSeconds` _cursimtime))))
  (if (`self.tryingToWalkTo_START`)
    (bind _output_get (set `self.startPos` (.location (`self.GetTransform`))))
    (set `self.startWalkTime` (`/Game/Controller.curSimTime` _as_controller))
    (bind _output_get_2 (set `self.secondsToReachPoint` (/ (`KismetMathLibrary.Vector_Distance` _output_get _go_to) 150.0)))
    (set `self.tryingToWalkTo_START` false)
    (set `self.walking` true)
    (elif (`self.walking`)
      (bind _returnvalue (/ (`KismetMathLibrary.GetTotalSeconds` (- _cursimtime (`self.startWalkTime`))) _output_get_2))
      (if (>= _returnvalue 1.0)
        (`self.K2_SetActorLocationAndRotation` _go_to)
        (set `self.walking` false)
        (else
          (`self.K2_SetActorLocationAndRotation` (`KismetMathLibrary.VLerp` (`self.startPos`) _go_to _returnvalue))))))
  (`/Game/simSteps/a1/simManaged2.SimStep completed` (`self.simManaged2`)))

(event `DoWalkToPoint`
  (params (goTo :type "Vector Structure"))
  (set `self.Go To` goTo)
  (set `self.tryingToWalkTo_START` true))

(fn `UserConstructionScript`)