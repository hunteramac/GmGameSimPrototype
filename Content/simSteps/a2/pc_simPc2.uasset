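; Simulated actor (pc_simPc2) that sweeps along a path of points and stops early when it perceives the actor it is looking for.
; FWalkAlong lerps its transform toward each point in SimDistStep-sized increments within a single call, with no Tick or timing, printing positions.
; After each move, CheckForPercepts tests whether LookingFor is valid and within a fixed radius; a hit aborts the walk and returns false.
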(event `self.ReceiveTick`
  (params (DeltaSeconds :type "Float (single-precision)")))

(fn `CheckForPercepts`
  (returns (perceptDetected :type Boolean))
  (`/Engine/EditorBlueprintResources/StandardMacros.IsValid` (`self.LookingFor`)
    (:`Is Valid`
      (if (<= (`KismetMathLibrary.Vector_Distance` (.location (`self.GetTransform` (`self.LookingFor`))) (.location (`self.GetTransform`))) 500.0)
        (return true)
        (else
          _)))
    (:`Is Not Valid`
      _))
  (return false))

(fn `fWalkAlong`
  (params (path :type "Array of Vector Structure") (simDistStep :type "Float (double-precision)"))
  (returns (finSuccess :type Boolean))
  (locals (NewLocalVar :type "Vector Structure" :default (0.0 0.0 0.0)) (NewLocalVar_0 :type "Float (single-precision)" :default 0.0))
  (for _array_element path
    (bind _output_get (set `local.NewLocalVar` (.location (`self.GetTransform`)))) ; get starting transform
    (set `local.NewLocalVar_0` 0.0)
    (while (<= (`local.NewLocalVar_0`) 1.0)
      (bind _returnvalue (`KismetMathLibrary.VLerp` _output_get _array_element (`local.NewLocalVar_0`)))
      (`self.K2_SetActorLocationAndRotation` _returnvalue)
      (bind _perceptdetected (`self.CheckForPercepts`))
      (if _perceptdetected
        (`KismetSystemLibrary.PrintText` "Intterupt occured during sweep")
        (return false)
        (else
          (set `local.NewLocalVar_0` (+ (`local.NewLocalVar_0`) (/ 1.0 (/ (`KismetMathLibrary.Vector_Distance` _output_get _array_element) simDistStep))))
          (`KismetSystemLibrary.PrintText` (`|FormatText` "x {1} y {2} z {3}" (.x _returnvalue) (.y _returnvalue) (.z _returnvalue))))))
    (`KismetSystemLibrary.PrintText` "do next path"))
  (return true))

(fn `UserConstructionScript`)