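; Gunslinger portrayal Blueprint that shows a given state as a frozen pose on the Gunslinger mesh.
; Its PortrayState override calls DoPortray, which looks up the first state entry's Type in the GunslingerAnims map for an animation and time frame.
; It plays the animation, jumps to that time with notifies firing, then stops to hold the pose.
; An earlier data-table lookup remains disconnected, noted as a maintenance burden.
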(event `doPortray`
  (params (state :type "Array of /Game/figuringOutDoing/statePercept Structure"))
  (bind _gunslinger (`self.gunslinger`))
  (bind (_value _returnvalue) (`BlueprintMapLibrary.Map_Find` (`PortrayalProfile.Animations` (`self.gunslingerAnims`)) (`.type_2_F85AF96F4685C6B51BDB6DB636D9DE3C` (break `/Game/figuringOutDoing/statePercept` (`|GetArrayItem` state)))))
  (bind (_animation _timeframe) (break `AnimFrame` _value))
  (if _returnvalue
    (`SkeletalMeshComponent.PlayAnimation` _gunslinger _animation false)
    (`SkeletalMeshComponent.SetPosition` _gunslinger _timeframe true)
    (`SkeletalMeshComponent.Stop` (`self.gunslinger`))))

(fn `portrayState`
  (params (state :type "Array of /Game/figuringOutDoing/statePercept Structure (by ref)"))
  (`self.doPortray` state)
  (return))

(fn `UserConstructionScript`)