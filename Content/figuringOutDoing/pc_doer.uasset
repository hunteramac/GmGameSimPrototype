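; Doer Blueprint that holds a current action to pursue and periodically reports its type as debug text.
; SetAction replaces the stored action, whose Type is Stand, Run or Walk.
; Tick accumulates delta time through the same path for every type, then prints the matching state every five seconds and resets the timer.
; No movement or other behavior is implemented yet.
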(event `self.ReceiveTick`
  (params (DeltaSeconds :type "Float (single-precision)"))
  (bind _topursue (`self.toPursue`))
  (switch `/Game/ActionExecution/E_actionType_gunslinger` (`.type_6_9EA34BBC44582F503900FDBBCD37A880` (break `/Game/ActionExecution/S_DeclaredActionInfo` _topursue))
    (:`NewEnumerator1`
      _)
    (:`NewEnumerator2`
      _)
    (:`NewEnumerator3`
      _))
  (bind _output_get (set `self.timeDiff` (+ DeltaSeconds (`self.timeDiff`))))
  (if (> _output_get 5.0)
    (set `self.timeDiff` 0.0)
    (switch `/Game/ActionExecution/E_actionType_gunslinger` (`.type_6_9EA34BBC44582F503900FDBBCD37A880` (break `/Game/ActionExecution/S_DeclaredActionInfo` _topursue))
      (:`NewEnumerator1`
        (`KismetSystemLibrary.PrintText` "standing"))
      (:`NewEnumerator2`
        (`KismetSystemLibrary.PrintText` "running"))
      (:`NewEnumerator3`
        (`KismetSystemLibrary.PrintText` "walking")))))

(event `SetAction`
  (params (newAction :type "/Game/ActionExecution/S_DeclaredActionInfo Structure"))
  (set `self.toPursue` newAction))

(fn `UserConstructionScript`)