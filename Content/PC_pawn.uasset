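; PC_pawn is a pawn with placeholder movement and a simple perception memory.
; Walk requests store a target that Tick hands to a handler, which teleports there instead of walking.
; Walk-along requests teleport to the nearest point on the supplied spline as a proof of concept, printing both positions.
; Percepts accumulate uniquely in SenseList, and those flagged MAWorthy fire the MAWorthyPerceptDetected dispatcher.
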(event `self.ReceiveTick`
  (params (DeltaSeconds :type "Float (single-precision)"))
  (if (`self.tryingToWalkTo`)
    (`self.handle walk to`)))

(event `handle walk to`
  (`self.K2_TeleportTo` (`self.walkToTarget`)) ; just teleport for now
  (set `self.tryingToWalkTo` false))

(fn `AddPercept`
  (params (NewParam :type "/Game/percept Structure"))
  (`KismetArrayLibrary.Array_AddUnique` (`self.senseList`) NewParam)
  (if (`.MA_Worthy?_10_AF545F204D441A54BE9B7E94ED412325` (break `/Game/percept` NewParam))
    (`self.MA_WorthyPerceptDetected`)))

(fn `GetPercepts`
  (returns (NewParam :type "Array of /Game/percept Structure"))
  (return (`self.senseList`)))

(fn `StartWalkAlong`
  (params (NewParam :type "SplineComponent Object Reference"))
  (bind _location (.location (`self.GetTransform`)))
  (bind _location_2 (.location (`SplineComponent.FindTransformClosestToWorldLocation` NewParam _location "World" false)))
  ; Just teleport to closest point, as proof we can use splines
  (`KismetSystemLibrary.PrintText` (`|FormatText` "X: {0} Y: {1} Z: {2}" (.x _location) (.y _location) (.z _location)))
  (`KismetSystemLibrary.PrintText` (`|FormatText` "X: {0} Y: {1} Z: {2}" (.x _location_2) (.y _location_2) (.z _location_2)))
  (`self.K2_TeleportTo` _location_2))

(fn `startWalkTo`
  (params (waltToTarget :type "Vector Structure"))
  (set `self.tryingToWalkTo` true)
  (set `self.walkToTarget` waltToTarget))

(fn `UserConstructionScript`)