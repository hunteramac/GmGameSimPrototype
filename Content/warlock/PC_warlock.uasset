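; Warlock actor Blueprint that turns what it senses and does into timeline-ready "game percepts" and can travel along a road spline.
; AI perception updates become percepts from each actor's Descript component, stamped with the player controller's sim time.
; AddPercept stores them uniquely in PerceptList and calls PerceptLogged.
; FollowSpline moves the warlock via a duration-scaled Timeline, logging a departure percept and a hardcoded Brenfelt arrival percept.
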(event `self.ReceiveBeginPlay`)

(event `self.AIPerception.OnPerceptionUpdated`
  (params (UpdatedActors :type "Array of Actor Object Reference (by ref)"))
  ; Convert AI senses to 'game percepts'
  (for _array_element UpdatedActors
    (bind _returnvalue (`self.GetComponentByClass` _array_element "/Game/warlock/descript.descript_C"))
    (`/Engine/EditorBlueprintResources/StandardMacros.IsValid` _returnvalue
      (:`Is Valid`
        (bind _ascontroller (cast `/Game/Controller` (`GameplayStatics.GetPlayerController` 0)))
        (`self.Add percept` (make `/Game/percept_v2` true (`/Game/warlock/descript.shortDesc` _returnvalue) (make `/Game/timeRange` (`/Game/Controller.curSimTime` _ascontroller)) (`|MakeArray` _array_element)))))))

(event `Add percept`
  (params (NewItem :type "/Game/percept_v2 Structure (by ref)"))
  (bind _perceptlist (`self.perceptList`))
  (bind _returnvalue (`KismetArrayLibrary.Array_AddUnique` _perceptlist NewItem))
  (if (`KismetArrayLibrary.Array_IsValidIndex` _perceptlist _returnvalue)
    (`self.perceptLogged`)))

(event `FollowSpline`
  (params (`spline component` :type "SplineComponent Object Reference") (`time in seconds to complete following spline` :type "Float (double-precision)"))
  (`self.Add percept` (make `/Game/percept_v2` false "The Warlock walks down the road." (struct :`start` "+00000000.00:00:00.000000000" :`end` "+00000000.00:00:00.000000000") (`|MakeArray` (`ActorComponent.GetOwner` `spline component`))))
  (`TimelineComponent.SetPlayRate` (`self.my timeline`) (/ 1.0 `time in seconds to complete following spline`))
  (bind (_direction _newtrack_0) (`Timeline|my timeline`)
    (:`Update`
      (bind _returnvalue (`KismetMathLibrary.Lerp` 0.0 (`SplineComponent.GetSplineLength` `spline component`) _newtrack_0))
      (`self.K2_SetActorLocationAndRotation` (`SplineComponent.GetLocationAtDistanceAlongSpline` `spline component` _returnvalue "World") (`SplineComponent.GetRotationAtDistanceAlongSpline` `spline component` _returnvalue "World")))
    (:`Finished`
      ; HARDCODED percept
      (`self.Add percept` (make `/Game/percept_v2` true "The warlock reaches Brenfelt midmorning, 2 days after setting off from Earnstead.")))))

(fn `UserConstructionScript`)