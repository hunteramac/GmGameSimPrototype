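; PC_perceiver is a player-character actor that records percepts of its own activity and can travel along a spline.
; makePercept adds a percept holding itself, its transform and current Doing state to a list, then calls PCPerceivedAThing.
; FollowSpline teleports to the spline start and moves along it by timeline over a given duration, changing Doing and recording a percept at both ends.
; The AI perception update handler is empty.
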(event `self.AIPerception.OnPerceptionUpdated`
  (params (UpdatedActors :type "Array of Actor Object Reference (by ref)")))

(event `makePercept`
  (`KismetArrayLibrary.Array_AddUnique` (`self.perceptListV5`) (make `/Game/portrayingPercepts/Percept_v5_doing` self (`self.GetTransform`) (`self.doing`)))
  (`self.PC perceived a thing`))

(event `FollowSpline`
  (params (`spline component` :type "SplineComponent Object Reference") (`time in seconds to complete following spline` :type "Float (double-precision)"))
  (set `self.doing` "NewEnumerator1")
  (`self.K2_TeleportTo` self (`SplineComponent.GetLocationAtDistanceAlongSpline` `spline component` 0.0 "World") (`SplineComponent.GetRotationAtDistanceAlongSpline` `spline component` 0.0 "World"))
  (`self.makePercept`)
  (`TimelineComponent.SetPlayRate` (`self.Timeline`) (/ 1.0 `time in seconds to complete following spline`))
  (bind (_direction _newtrack_0) (`Timeline|Timeline`)
    (:`Update`
      (bind _returnvalue (`KismetMathLibrary.Lerp` 0.0 (`SplineComponent.GetSplineLength` `spline component`) _newtrack_0))
      (`self.K2_SetActorLocationAndRotation` (`SplineComponent.GetLocationAtDistanceAlongSpline` `spline component` _returnvalue "World") (`SplineComponent.GetRotationAtDistanceAlongSpline` `spline component` _returnvalue "World")))
    (:`Finished`
      (set `self.doing` "NewEnumerator0")
      (`self.makePercept`))))

(fn `UserConstructionScript`)